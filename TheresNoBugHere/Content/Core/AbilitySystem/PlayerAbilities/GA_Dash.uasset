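; Player dash Gameplay Ability that turns the avatar toward its last movement direction and plays a dash montage.
; On activation it adds a BlockMove state tag, snaps the actor's rotation, then plays the montage looked up by gameplay tag.
; Any montage outcome (completed, blend out, interrupted or cancelled) ends the ability, and OnEndAbility removes the BlockMove tag.
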(event Ability|EventActivateAbility
  (bind _returnvalue (Ability|GetActorInfo))
  (|CallParentFunction)
  (Class|NBGamePlayFunctionLibrary|AddStateTag (.avataractor _returnvalue) "(TagName=\"NB_Tags.State.BlockMove\")")
  (Transformation|SetActorRotation (.avataractor _returnvalue) (Math|Rotator|MakeRotfromXZ (Class|NBGamePlayFunctionLibrary|GetLastMovementWorldDirection (.avataractor _returnvalue)) (Math|Vector|MakeVector 0.0 0.0 1.0)))
  (|PlayMontageandWaitProxy "None" (Class|UNBAnimationFunctionLibrary|GetMontagebyTag (.avataractor _returnvalue) "(TagName=\"NB_Tags.Animation.Montage.Dash\")") 1.0 "None" true 1.0 0.0 false
    (:OnCompleted
      _)
    (:OnBlendOut
      _)
    (:OnInterrupted
      _)
    (:OnCancelled
      _))
  (Ability|EndAbility self))

(event Ability|EventOnEndAbility
  (params (bWasCancelled :type Boolean))
  (|CallParentFunction bWasCancelled)
  (Class|NBGamePlayFunctionLibrary|RemoveStateTag (.avataractor (Ability|GetActorInfo)) "(TagName=\"NB_Tags.State.BlockMove\")"))